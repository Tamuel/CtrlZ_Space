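; Food item Blueprint in the space game that tracks a food resource amount inside its ItemData structure.
; GetResource rebuilds the structure with the Food value added to Amount and marks it as owned.
; ReduceResource subtracts Supply from Amount without a floor check, then re-arms itself by name on a 50-second timer, creating recurring consumption once triggered.
; BeginPlay, overlap and Tick are empty.
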(event EventBeginPlay)

(event EventActorBeginOverlap
  (params (OtherActor :type Actor%20Object%20Reference)))

(event EventTick
  (params (DeltaSeconds :type Float%20%28single-precision%29)))

(event EventGetResource
  (Variables|Default|SetitemData (Utilities|Struct|MakeItemStructure (.name (Utilities|Struct|BreakItemStructure (Variables|Default|GetitemData))) (.Price (Utilities|Struct|BreakItemStructure (Variables|Default|GetitemData))) (.weight (Utilities|Struct|BreakItemStructure (Variables|Default|GetitemData))) (+ (.amount (Utilities|Struct|BreakItemStructure (Variables|Default|GetitemData))) (Variables|Default|Getfood)) true)))

(event EventReduceResource
  (Variables|Default|SetitemData (Utilities|Struct|MakeItemStructure (.name (Utilities|Struct|BreakItemStructure (Variables|Default|GetitemData))) (.Price (Utilities|Struct|BreakItemStructure (Variables|Default|GetitemData))) (.weight (Utilities|Struct|BreakItemStructure (Variables|Default|GetitemData))) (- (.amount (Utilities|Struct|BreakItemStructure (Variables|Default|GetitemData))) (Variables|Default|Getsupply)) (.owner (Utilities|Struct|BreakItemStructure (Variables|Default|GetitemData)))))
  (Utilities|Time|SetTimerbyFunctionName 0 "reduceResource" 5e+01))

(fn ConstructionScript
  (|CallParentFunction))