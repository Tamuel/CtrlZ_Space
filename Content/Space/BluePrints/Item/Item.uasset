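; Item actor that shows a pickup widget when a player unit walks into it while the item is unowned.
; On overlap it checks that the actor's Owner is unset and the other actor is a player Unit, then creates, stores and displays a GetItemWidget.
; SetItemOwner rebuilds the ItemData struct with the given Unit as owner, leaving the actor's own Owner untouched.
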(event EventBeginPlay)

(event EventActorBeginOverlap
  (params (OtherActor :type Actor%20Object%20Reference))
  (Utilities|IsValid (Components|GetOwner self)
    (:Is%20Not%20Valid
      (bind _asunit (Utilities|Casting|CastToUnit OtherActor))
      (if (Variables|/Game/Space/BluePrints/Unit/Unit.Unit_C|GetisPlayer _asunit)
        (bind _returnvalue (UserInterface|CreateWidget "/Game/Space/BluePrints/Item/widget/getItemWidget.getItemWidget_C"))
        (bind _output_get (Variables|Default|SetgetItemWidget _returnvalue))
        (UserInterface|Viewport|AddtoViewport _output_get 0)))))

(event EventTick
  (params (DeltaSeconds :type Float%20%28single-precision%29)))

(fn ConstructionScript)

(fn SetItemOwner
  (params (Unit :type Unit%20Object%20Reference))
  (Variables|Default|SetitemData (Utilities|Struct|MakeItemStructure (.name (Utilities|Struct|BreakItemStructure (Variables|Default|GetitemData))) (.Price (Utilities|Struct|BreakItemStructure (Variables|Default|GetitemData))) (.weight (Utilities|Struct|BreakItemStructure (Variables|Default|GetitemData))) (.amount (Utilities|Struct|BreakItemStructure (Variables|Default|GetitemData))) Unit)))