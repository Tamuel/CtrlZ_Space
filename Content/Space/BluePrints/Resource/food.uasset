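; Food resource Blueprint that tracks a stock of food which drains over time.
; BeginPlay seeds the ResourceData struct with a name and starting amount, then starts consumption.
; SpendResource subtracts Supply and re-arms itself on a one-minute timer by function name, forming a repeating drain.
; GetResource adds Survivor to the amount, rebuilding the struct with the same name and owner.
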(event EventBeginPlay
  (Variables|Default|SetresourceData (Utilities|Struct|MakeresourceStructure "food" 100))
  (CallFunction|SpendResource))

(event Collision|EventActorBeginOverlap
  (params (OtherActor :type Actor%20Object%20Reference)))

(event EventGetResource
  (Variables|Default|SetresourceData (Utilities|Struct|MakeresourceStructure (.name (Utilities|Struct|BreakresourceStructure (Variables|Default|GetresourceData))) (+ (.amount (Utilities|Struct|BreakresourceStructure (Variables|Default|GetresourceData))) (Variables|Default|Getsurvivor)) (.owner (Utilities|Struct|BreakresourceStructure (Variables|Default|GetresourceData))))))

(event EventSpendResource
  (Variables|Default|SetresourceData (Utilities|Struct|MakeresourceStructure (.name (Utilities|Struct|BreakresourceStructure (Variables|Default|GetresourceData))) (- (.amount (Utilities|Struct|BreakresourceStructure (Variables|Default|GetresourceData))) (Variables|Default|Getsupply)) (.owner (Utilities|Struct|BreakresourceStructure (Variables|Default|GetresourceData)))))
  (Utilities|Time|SetTimerbyFunctionName 0 "spendResource" 6e+01))

(event EventTick
  (params (DeltaSeconds :type Float%20%28single-precision%29)))

(fn ConstructionScript
  (|CallParentFunction))