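; Cursor actor for the space planet node map that starts hovering slightly above its start node and glides to a target position.
; On BeginPlay it teleports to just above PStartNode.
; While IsMoving is set, Tick faces it toward ToPosition and advances it along local X by a fraction of the remaining distance, easing out per frame.
; Once nearly there, it snaps to ToPosition and clears IsMoving.
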(event EventBeginPlay
  (bind _pstartnode (Variables|Default|GetPStartNode))
  (bind _returnvalue (Transformation|GetActorLocation _pstartnode))
  (bind (_x _y _z) (Math|Vector|BreakVector _returnvalue))
  ;[1 1 1] When game start, Cursor's position in startNode.
  (Transformation|SetActorLocation (Math|Vector|MakeVector _x _y (+ _z 12.0)) false false))

(event Collision|EventActorBeginOverlap
  (params (OtherActor :type Actor%20Object%20Reference)))

(event EventTick
  (params (DeltaSeconds :type Float%20%28single-precision%29))
  (bind _self self)
  (bind _toposition (Variables|Default|GetToPosition))
  (bind _returnvalue (Transformation|GetActorLocation _self))
  (bind _returnvalue_2 (- _toposition _returnvalue))
  (bind _returnvalue_3 (Math|Vector|VectorLength _returnvalue_2))
  ;[1 1 1] Go to ToPosition
  (if (Variables|Default|GetIsMoving)
    (if (> _returnvalue_3 0.1)
      (Transformation|SetActorRotation (Math|Rotator|MakeRotfromX _returnvalue_2))
      (Transformation|AddActorLocalOffset (Math|Vector|MakeVector (/ _returnvalue_3 1e+01) 0.0 0.0) false false)
      (else
        ;[1 1 1] Stop Move
        (Variables|Default|SetIsMoving false)
        (Transformation|SetActorLocation self (Variables|Default|GetToPosition) false false)))))

(fn ConstructionScript)