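; Iron resource item Blueprint that tracks the player's iron as an item data struct.
; GetResource adds the weight and amount of the GetIron item when iron is acquired.
; ReduceResource handles purchases, subtracting the BuyItem's weight from iron weight and its price from iron amount.
; Both events rebuild the struct, preserving the other fields; the default events are empty and construction defers to the parent.
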(event EventBeginPlay)

(event EventActorBeginOverlap
  (params (OtherActor :type Actor%20Object%20Reference)))

(event EventTick
  (params (DeltaSeconds :type Float%20%28single-precision%29)))

(event EventGetResource
  ;[1 1 1] Iron 획득 시
  (Variables|Default|SetitemData (Utilities|Struct|MakeItemStructure (.name (Utilities|Struct|BreakItemStructure (Variables|Default|GetitemData))) (.Price (Utilities|Struct|BreakItemStructure (Variables|Default|GetitemData))) (+ (.weight (Utilities|Struct|BreakItemStructure (Variables|Default|GetitemData))) (.weight (Utilities|Struct|BreakItemStructure (Variables|/Game/Space/BluePrints/Item/Item.Item_C|GetitemData (Variables|Default|GetgetIron))))) (+ (.amount (Utilities|Struct|BreakItemStructure (Variables|Default|GetitemData))) (.amount (Utilities|Struct|BreakItemStructure (Variables|/Game/Space/BluePrints/Item/Item.Item_C|GetitemData (Variables|Default|GetgetIron))))) (.image (Utilities|Struct|BreakItemStructure (Variables|Default|GetitemData))) (.owner (Utilities|Struct|BreakItemStructure (Variables|Default|GetitemData))))))

(event EventReduceResource
  ;[1 1 1] Iron을 사용해 아이템 구매
  (Variables|Default|SetitemData (Utilities|Struct|MakeItemStructure (.name (Utilities|Struct|BreakItemStructure (Variables|Default|GetitemData))) (.Price (Utilities|Struct|BreakItemStructure (Variables|Default|GetitemData))) (- (.weight (Utilities|Struct|BreakItemStructure (Variables|Default|GetitemData))) (.weight (Utilities|Struct|BreakItemStructure (Variables|/Game/Space/BluePrints/Item/Item.Item_C|GetitemData (Variables|Default|GetbuyItem))))) (- (.amount (Utilities|Struct|BreakItemStructure (Variables|Default|GetitemData))) (.Price (Utilities|Struct|BreakItemStructure (Variables|/Game/Space/BluePrints/Item/Item.Item_C|GetitemData (Variables|Default|GetbuyItem))))) (.image (Utilities|Struct|BreakItemStructure (Variables|Default|GetitemData))) (.owner (Utilities|Struct|BreakItemStructure (Variables|Default|GetitemData))))))

(fn ConstructionScript
  (|CallParentFunction))