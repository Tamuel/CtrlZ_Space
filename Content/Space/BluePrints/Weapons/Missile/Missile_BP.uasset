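; Missile weapon projectile that flies forward under axis-input steering and damages Destroyable actors it overlaps.
; Axis inputs adjust clamped forward and yaw speeds, with turning easing off without input, and Tick applies them as swept local movement.
; Overlaps skip the owner and its attached units, apply Power damage, then detonate.
; A hit or lifetime timer stops and hides the missile, spawns particles, and destroys it when they finish.
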(event Custom|DestroyEvent
  ;[1 1 1] Destroy Event
  (Class|KismetSystemLibrary|ClearTimerHandle (Variables|Default|GetDestroyTimerHandler))
  (Variables|Properties|SetCurrentForwardSpeed 0.0)
  (Variables|Properties|SetAcceleration 0.0)
  (Variables|Properties|SetTurningSpeed 0.0)
  (Variables|Properties|SetCurrentTurningSpeed 0.0)
  (bind _returnvalue (AddComponent|AddParticleSystemComponent false))
  (Class|Pawn|DetachfromControllerPendingDestroy)
  (EventDispatchers|AssignOnSystemFinished _returnvalue (delegate Custom|OnSystemFinished_이벤트_0))
  (Rendering|SetVisibility (Variables|Default|GetMissile1_) false false))

(event Custom|OnSystemFinished_이벤트_0
  (params (PSystem :type Particle%20System%20Component%20Object%20Reference))
  ;[1 1 1] Destroy Event
  (Actor|DestroyActor))

(event EventBeginPlay
  ;[1 1 1] When Game Begin
  (bind _returnvalue (Utilities|Time|SetTimerbyFunctionName 0 "Destroy" (Variables|Default|GetTime)))
  (Variables|Default|SetDestroyTimerHandler _returnvalue))

(event EventTick
  (params (DeltaSeconds :type Float%20%28single-precision%29))
  ;[1 1 1] Update in Each Frame
  (Transformation|AddActorLocalOffset (Math|Vector|MakeVector (* DeltaSeconds (Variables|Properties|GetCurrentForwardSpeed)) 0.0 0.0) true false)
  (Transformation|AddActorLocalRotation (Math|Rotator|MakeRotator 0.0 0.0 (* (Utilities|Time|GetWorldDeltaSeconds) (Variables|Properties|GetCurrentTurningSpeed))) true false))

(event Collision|EventActorBeginOverlap
  (params (OtherActor :type Actor%20Object%20Reference))
  ;[1 1 1] When be Shot
  (bind _isenemy (CallFunction|DecideHitorNot OtherActor))
  (if _isenemy
    (bind _asdestroyable (Utilities|Casting|CastToDestroyable OtherActor))
    (if (not (== (Variables|/Game/Space/BluePrints/Destroyable/Destroyable.Destroyable_C|GetCurrentDurability _asdestroyable) 0))
      (Default|Damaged _asdestroyable (Variables|Default|GetPower) (Transformation|GetActorLocation self) (Variables|Default|GetOwnerOfWeapon))
      (AddComponent|AddAudioComponent false)
      (CallFunction|DestroyEvent)
      (Variables|Default|SetDisableBullet true))))

(event Input|AxisEvents|InputAxisForwardAndBackward
  (params (AxisValue :type Float%20%28single-precision%29))
  ;[1 1 1] Move Forward or Backward, Speed Not Decrease when input disable
  (CallFunction|MoveForwardorBackward AxisValue))

(event Input|AxisEvents|InputAxisLeftAndRight
  (params (AxisValue :type Float%20%28single-precision%29))
  ;[1 1 1] Turn Left or Right, Rotation speed is decrease when input disable
  (CallFunction|TurnLeftorRight AxisValue))

(fn ConstructionScript)

(fn TurnLeftorRight
  (params (AxisValue :type Float%20%28single-precision%29))
  (bind _returnvalue (Utilities|Time|GetWorldDeltaSeconds))
  (bind _turningspeed (Variables|Properties|GetTurningSpeed))
  ;[1 1 1] Turn Left or Right, If no input than rotation speed is decrease.
  (Variables|Properties|SetCurrentTurningSpeed (Math|Float|SelectFloat (Math|Float|SelectFloat (+ (Variables|Properties|GetCurrentTurningSpeed) (* _returnvalue (* _turningspeed 0.7))) (+ (Variables|Properties|GetCurrentTurningSpeed) (* _returnvalue (* _turningspeed -0.7))) (<= (Variables|Properties|GetCurrentTurningSpeed) 0.0)) (Math|Float|Clamp(Float) (+ (* (* AxisValue _turningspeed) _returnvalue) (Variables|Properties|GetCurrentTurningSpeed)) (Variables|Properties|GetMinTurnSpeed) (Variables|Properties|GetMaxTurnSpeed)) (== AxisValue 0.0))))

(fn MoveForwardorBackward
  (params (AxisValue :type Float%20%28single-precision%29))
  ;[1 1 1] Move Forward or Backward, Speed Not Decrease when no input
  (Variables|Properties|SetCurrentForwardSpeed (Math|Float|Clamp(Float) (+ (Variables|Properties|GetCurrentForwardSpeed) (* (Utilities|Time|GetWorldDeltaSeconds) (* AxisValue (Variables|Properties|GetAcceleration)))) (Variables|Properties|GetMinSpeed) (Variables|Properties|GetMaxSpeed))))

(fn Destroy
  (CallFunction|DestroyEvent))

(fn DecideHitorNot
  (params (OtherActor :type Actor%20Object%20Reference))
  (bind _ownerofweapon (Variables|Default|GetOwnerOfWeapon))
  (bind _asunit_attachable (Utilities|Casting|CastToUnitAttachable OtherActor)
    (:then
      (if (!= _ownerofweapon (Variables|/Game/Space/BluePrints/Unit/UnitAttachable.UnitAttachable_C|GetOwnerUnit _asunit_attachable))
        _
        (else
          (return false))))
    (:CastFailed
      (if (!= OtherActor _ownerofweapon)
        _
        (else
          (return false)))))
  (return (and (Utilities|ClassIsChildOf (Utilities|GetClass OtherActor) "/Game/Space/BluePrints/Destroyable/Destroyable.Destroyable_C") (not (Variables|Default|GetDisableBullet)))))