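; itemView is a world pickup actor that represents an item the player can collect in the space game.
; On BeginPlay it spawns an actor of its ItemClass, initializes it and attaches it to itself.
; When a player Unit overlaps it, it adds a GetItem widget to that player's interaction list, removing it when the overlap ends.
; RemoveItemView destroys both the item and the view.
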(event Collision|EventActorBeginOverlap
  (params (OtherActor :type Actor%20Object%20Reference))
  ;[1 1 1] PlayerShip과 Item이 겹쳐졌을 시 획득 여부를 묻는 위젯을 띄움
  (bind _asunit (Utilities|Casting|CastToUnit OtherActor))
  (if (Variables|/Game/Space/BluePrints/Unit/Unit.Unit_C|GetisPlayer _asunit)
    (bind _returnvalue (UserInterface|CreateWidget "/Game/Space/BluePrints/Item/widget/getItemWidget.getItemWidget_C"))
    (bind _output_get (Variables|Default|SetgetItemWidget _returnvalue))
    (Utilities|Array|Add (Variables|/Game/Space/BluePrints/Player/SpacePlayer.SpacePlayer_C|GetInteractionWidgets (Variables|/Game/Space/BluePrints/Unit/Unit.Unit_C|GetPlayer _asunit)) _output_get)
    (Variables|/Game/Space/BluePrints/Item/widget/getItemWidget.getItemWidget_C|SetgetItemWidgetItem (Variables|Default|GetgetItemWidget) (Variables|Default|Getitem))
    (Variables|/Game/Space/BluePrints/Item/widget/getItemWidget.getItemWidget_C|SetgetItemWidgetUnit (Variables|Default|GetgetItemWidget) _asunit)
    (Variables|/Game/Space/BluePrints/Item/widget/getItemWidget.getItemWidget_C|SetgetItemWidgetItemView (Variables|Default|GetgetItemWidget) self)))

(event Collision|EventActorEndOverlap
  (params (OtherActor :type Actor%20Object%20Reference))
  (bind _getitemwidget (Variables|Default|GetgetItemWidget))
  (bind _asunit (Utilities|Casting|CastToUnit OtherActor))
  (if (Variables|/Game/Space/BluePrints/Unit/Unit.Unit_C|GetisPlayer _asunit)
    (if (== (Variables|/Game/Space/BluePrints/Player/SpacePlayer.SpacePlayer_C|GetCurrentInteractionUI (Variables|/Game/Space/BluePrints/Unit/Unit.Unit_C|GetPlayer _asunit)) _getitemwidget)
      (Variables|/Game/Space/BluePrints/Player/SpacePlayer.SpacePlayer_C|SetInteractionUIIsOn (Variables|/Game/Space/BluePrints/Unit/Unit.Unit_C|GetPlayer _asunit) false))
    (Utilities|Array|RemoveItem (Variables|/Game/Space/BluePrints/Player/SpacePlayer.SpacePlayer_C|GetInteractionWidgets (Variables|/Game/Space/BluePrints/Unit/Unit.Unit_C|GetPlayer _asunit)) _getitemwidget)
    (Widget|RemovefromParent (Variables|Default|GetgetItemWidget))))

(event EventBeginPlay
  (CallFunction|MakeItem))

(event EventTick
  (params (DeltaSeconds :type Float%20%28single-precision%29)))

(fn ConstructionScript)

(fn MakeItem
  (bind _returnvalue (Game|SpawnActorfromClass (Variables|Default|GetitemClass) (Math|Transform|MakeTransform "0, 0, 0") "AlwaysSpawn" 0 0))
  (bind _output_get (Variables|Default|Setitem _returnvalue))
  (Utilities|IsValid _output_get
    (:Is%20Valid
      (Default|InitializeItem _output_get)
      (Class|Actor|AttachRootComponenttoActor _output_get self "None" "SnapToTarget" true))))

(fn RemoveItemView
  (Actor|DestroyActor (Variables|Default|Getitem))
  (Actor|DestroyActor))