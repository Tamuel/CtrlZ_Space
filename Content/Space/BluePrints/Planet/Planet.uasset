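; Planet is a space-map actor that moves the player into a planet level when their ship touches it.
; On overlap with a player Unit, it creates a new SpaceSaveGame and stores the controlled SpacePlayer's OwnUnit in it.
; It writes that save to a temporary slot, then opens the PlanetOne level, whose name is hard-coded.
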(event EventBeginPlay)

(event Collision|EventActorBeginOverlap
  (params (OtherActor :type Actor%20Object%20Reference))
  ;[1 1 1] 행성이랑 ship이 overlap되었을 시 ship 데이터를 저장하고 레벨 호출
  (bind _asunit (Utilities|Casting|CastToUnit OtherActor))
  (if (Variables|/Game/Space/BluePrints/Unit/Unit.Unit_C|GetisPlayer _asunit)
    (bind _returnvalue (SaveGame|CreateSaveGameObject "/Game/Space/BluePrints/SaveGame/SpaceSaveGame.SpaceSaveGame_C"))
    (bind _asspace_save_game (Utilities|Casting|CastToSpaceSaveGame _returnvalue))
    (bind _asspace_player (Utilities|Casting|CastToSpacePlayer (Pawn|GetControlledPawn (Game|GetPlayerController 0))))
    (Default|SaveUnit _asspace_save_game (Variables|/Game/Space/BluePrints/Player/SpacePlayer.SpacePlayer_C|GetOwnUnit _asspace_player))
    (SaveGame|SaveGametoSlot _asspace_save_game "Temp")
    (Game|OpenLevel(byName) "PlanetOne")))

(event EventTick
  (params (DeltaSeconds :type Float%20%28single-precision%29)))

(fn ConstructionScript)