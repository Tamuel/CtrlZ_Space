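; Space ship unit base that handles physics-driven movement, damage, energy and skills.
; Axis inputs adjust clamped forward and turning speeds, with only turning decaying without input; Tick applies both as impulses to PhysicsCore, scaled by actor scale squared.
; Damage drains energy or durability by flag, calling an empty DestroyEvent at zero durability, while energy recharges unless draining.
; InitializeUnit spawns attached skill actors; UseSkill spends energy to activate the first, or re-triggers it if active.
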(event Custom|DestroyEvent)

(event EventTick
  (params (DeltaSeconds :type Float%20%28single-precision%29))
  (bind _self self)
  (bind _self_2 self)
  (bind _returnvalue (Transformation|GetActorScale3D _self))
  (bind _returnvalue_2 (Transformation|GetActorScale3D _self_2))
  (bind _x (Math|Vector|BreakVector _returnvalue))
  (bind _x_2 (Math|Vector|BreakVector _returnvalue_2))
  ;[1 1 1] Update in Each Frame
  (Physics|AddImpulse (Variables|Default|GetPhysicsCore) (* (* (Math|Vector|GetForwardVector (Variables|Default|GetPhysicsCore)) (* DeltaSeconds (Variables|Speed|GetCurrentForwardSpeed))) (* _x_2 _x_2)) "None" false)
  (Class|PrimitiveComponent|AddAngularImpulse (Variables|Default|GetPhysicsCore) (* (* (Math|Vector|MakeVector 0.0 0.0 (* (Utilities|Time|GetWorldDeltaSeconds) (Variables|Speed|GetCurrentTurningSpeed))) 1e+01) (* _x _x)) "None" false)
  (if (not (Variables|Default|GetDrainEnergy))
    (CallFunction|IncreaseEnergy)))

(event EventBeginPlay
  (Class|Actor|AttachRootComponentto (Variables|Default|GetPhysicsCore) "None" "KeepWorldPosition" true))

(event EventActorBeginOverlap
  (params (OtherActor :type Actor%20Object%20Reference)))

(event EventDamaged
  (params (Damage :type Integer) (Location :type Vector :default "0, 0, 0") (OtherActorsOwner :type Actor%20Object%20Reference))
  ;[1 1 1] Damaged
  (if (Variables|Default|GetDamageToEnergy)
    (CallFunction|DamagedonEnergy Damage)
    (else
      (CallFunction|DamagedonBody Damage))))

(event Input|AxisEvents|InputAxisLeftAndRight
  (params (AxisValue :type Float%20%28single-precision%29))
  ;[1 1 1] Turn Left or Right, Rotation speed is decrease when input disable
  (CallFunction|TurnLeftorRight AxisValue))

(event Input|AxisEvents|InputAxisForwardAndBackward
  (params (AxisValue :type Float%20%28single-precision%29))
  ;[1 1 1] Move Forward or Backward, Speed Not Decrease when input disable
  (CallFunction|MoveForwardorBackward AxisValue))

(fn ConstructionScript)

(fn TurnLeftorRight
  (params (Axis%20Value :type Float%20%28single-precision%29))
  (bind _returnvalue (Utilities|Time|GetWorldDeltaSeconds))
  (bind _turningspeed (Variables|Speed|GetTurningSpeed))
  (bind _maxturnspeed (Variables|Speed|GetMaxTurnSpeed))
  ;[1 1 1] Turn Left or Right, If no input than rotation speed is decrease.
  (Variables|Speed|SetCurrentTurningSpeed (Math|Float|SelectFloat (Math|Float|SelectFloat (+ (Variables|Speed|GetCurrentTurningSpeed) (* _returnvalue (* _turningspeed 0.8))) (+ (Variables|Speed|GetCurrentTurningSpeed) (* _returnvalue (* _turningspeed -0.8))) (<= (Variables|Speed|GetCurrentTurningSpeed) 0.0)) (Math|Float|Clamp(Float) (+ (* (* Axis%20Value _turningspeed) _returnvalue) (Variables|Speed|GetCurrentTurningSpeed)) (* _maxturnspeed -1.0) _maxturnspeed) (== Axis%20Value 0.0))))

(fn MoveForwardorBackward
  (params (AxisValue :type Float%20%28single-precision%29))
  ;[1 1 1] Move Forward or Backward, Speed Not Decrease when no input
  (Variables|Speed|SetCurrentForwardSpeed (Math|Float|Clamp(Float) (+ (Variables|Speed|GetCurrentForwardSpeed) (* (Utilities|Time|GetWorldDeltaSeconds) (* AxisValue (Variables|Speed|GetAcceleration)))) (Variables|Default|GetMinSpeed) (Variables|Default|GetMaxSpeed))))

(fn UseSkill
  (bind _skillsins (Variables|Default|GetSkillsIns))
  (bind _item (Utilities|Array|Get(acopy) _skillsins))
  (bind _skilldata (Variables|/Game/Space/BluePrints/Skills/Skill.Skill_C|GetSkillData _item))
  (bind (_cooltime _isactive _disable _energyconsumption) (Utilities|Struct|BreakSkillStructure _skilldata))
  (Utilities|IsValid _item
    (:Is%20Valid
      (if (not _disable)
        (if (and (>= (- (Variables|Default|GetCurrentEnergy) _energyconsumption) 0) (not _isactive))
          (Variables|Default|SetCurrentEnergy (- (Variables|Default|GetCurrentEnergy) _energyconsumption))
          (Default|ActiveSkill _item :!label _label)
          (elif _isactive
            (goto _label)))))))

(fn DamagedonBody
  (params (Damage :type Integer))
  ;[1 1 1] When Damaged On Ship, Set Text
  (bind _output_get (Variables|Default|SetCurrentDurability (- (Variables|Default|GetCurrentDurability) Damage)))
  (if (not (> _output_get 0))
    ;[1 1 1] Destroy Ship
    (Variables|Default|SetCurrentDurability 0)
    (CallFunction|DestroyEvent)))

(fn DamagedonEnergy
  (params (damage :type Integer))
  ;[1 1 1] When Damaged On Energy
  (bind _output_get (Variables|Default|SetCurrentEnergy (- (Variables|Default|GetCurrentEnergy) damage)))
  (if (< _output_get 0)
    _))

(fn DecreaseEnergy
  (params (energyDecreaseRate :type Integer))
  ;[1 1 1] Decrease Energy
  (bind _output_get (Variables|Default|SetCurrentEnergy (- (Variables|Default|GetCurrentEnergy) energyDecreaseRate)))
  (if (<= _output_get 0)
    (Variables|Default|SetCurrentEnergy 0)))

(fn IncreaseEnergy
  ;[1 1 1] Increase Energy
  (if (< (Variables|Default|GetCurrentEnergy) (Variables|Default|GetMaxEnergy))
    (bind _output_get (Variables|Default|SetCurrentEnergy (+ (Variables|Default|GetCurrentEnergy) (Variables|Default|GetEnergyChargeRate))))
    (if (> _output_get (Variables|Default|GetMaxEnergy))
      (Variables|Default|SetCurrentEnergy (Variables|Default|GetMaxEnergy)))))

(fn SetAlliance
  (params (Unit :type Unit%20Object%20Reference))
  (if (== (Variables|Default|GetAlliance) (Variables|Unit_C|GetAlliance Unit))
    (Utilities|Array|Add (Variables|Default|GetAlliances) Unit)))

(fn InitializeUnit
  ;[1 1 1] Initialize
  (Variables|Default|SetCurrentEnergy (Variables|Default|GetMaxEnergy))
  (for _array_element (Variables|Default|GetSkills)
    (bind _returnvalue (Game|SpawnActorfromClass _array_element (Math|Transform|MakeTransform (Transformation|GetActorLocation self)) "AlwaysSpawn" 0 0))
    (Variables|/Game/Space/BluePrints/Skills/Skill.Skill_C|SetSkillData _returnvalue "")
    (Class|Actor|AttachRootComponenttoActor _returnvalue self "None" "KeepWorldPosition" true)
    (Utilities|Array|Add (Variables|Default|GetSkillsIns) _returnvalue)))