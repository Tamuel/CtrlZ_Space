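; Iron resource Blueprint that holds the name, amount and owner of an iron stock in a resource structure.
; BeginPlay seeds the structure with the iron name and a starting amount.
; GetResource raises the amount by one and SpendResource subtracts ItemPrice with no balance check, each rebuilding the structure with name and owner preserved.
; Overlap and Tick are empty, and construction only calls the parent.
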(event EventBeginPlay
  (Variables|Default|SetresourceData (Utilities|Struct|MakeresourceStructure "iron" 100)))

(event EventTick
  (params (DeltaSeconds :type Float%20%28single-precision%29)))

(event Collision|EventActorBeginOverlap
  (params (OtherActor :type Actor%20Object%20Reference)))

(event EventGetResource
  (Variables|Default|SetresourceData (Utilities|Struct|MakeresourceStructure (.name (Utilities|Struct|BreakresourceStructure (Variables|Default|GetresourceData))) (+ (.amount (Utilities|Struct|BreakresourceStructure (Variables|Default|GetresourceData))) 1) (.owner (Utilities|Struct|BreakresourceStructure (Variables|Default|GetresourceData))))))

(event EventSpendResource
  (Variables|Default|SetresourceData (Utilities|Struct|MakeresourceStructure (.name (Utilities|Struct|BreakresourceStructure (Variables|Default|GetresourceData))) (- (.amount (Utilities|Struct|BreakresourceStructure (Variables|Default|GetresourceData))) (Variables|Default|GetitemPrice)) (.owner (Utilities|Struct|BreakresourceStructure (Variables|Default|GetresourceData))))))

(fn ConstructionScript
  (|CallParentFunction))