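; Blink skill for a ship, launching it in a fast dash toward a BlinkLocation actor when nothing overlaps that spot.
; ActiveSkill disables the skill for its cooldown, then applies a scale-adjusted physics impulse to HitPoint and spawns a directional particle.
; High linear damping brakes the dash until a short timer calls SetShipDamping to restore the lower value.
; Tick keeps the particle at the actor's location.
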(event EventBeginPlay)

(event Collision|EventActorBeginOverlap
  (params (OtherActor :type Actor%20Object%20Reference)))

(event EventTick
  (params (DeltaSeconds :type Float%20%28single-precision%29))
  (Utilities|IsValid (stale EventActiveSkill _returnvalue_7)
    (:Is%20Valid
      (Transformation|SetWorldLocation (stale EventActiveSkill _returnvalue_7) (Transformation|GetActorLocation 0) false false))))

(event EventActiveSkill
  (bind _returnvalue (Transformation|GetActorScale3D 0))
  (bind _blinklocation (Variables|/Game/Space/BluePrints/Ship/Ship.Ship_C|GetBlinkLocation 0))
  (bind _hitpoint (Variables|/Game/Space/BluePrints/Ship/Ship.Ship_C|GetHitPoint 0))
  (bind _x (Math|Vector|BreakVector _returnvalue))
  (bind _returnvalue_2 (Transformation|GetActorLocation _blinklocation))
  (bind _returnvalue_3 (Transformation|GetWorldLocation _hitpoint))
  (bind _returnvalue_4 (- _returnvalue_2 _returnvalue_3))
  (bind _returnvalue_5 (Math|Vector|Normalize _returnvalue_4))
  (if (== (Utilities|Array|Length (Collision|GetOverlappingActors (Variables|Default|GetBlinkLocation) "/Script/Engine.Actor" :!class /Script/Engine.Actor)) 0)
    (Variables|Default|SetSkillData (Utilities|Struct|MakeSkillStructure (.CoolTime (Utilities|Struct|BreakSkillStructure (Variables|Default|GetSkillData))) (.IsActive (Utilities|Struct|BreakSkillStructure (Variables|Default|GetSkillData))) true (.EnergyConsumption (Utilities|Struct|BreakSkillStructure (Variables|Default|GetSkillData))) (.Icon_Enable (Utilities|Struct|BreakSkillStructure (Variables|Default|GetSkillData))) (.Icon_Disable (Utilities|Struct|BreakSkillStructure (Variables|Default|GetSkillData))) (.Icon_On (Utilities|Struct|BreakSkillStructure (Variables|Default|GetSkillData)))))
    (bind _returnvalue_6 (Utilities|Time|SetTimerbyFunctionName 0 "EnableSkill" (.CoolTime (Utilities|Struct|BreakSkillStructure (Variables|Default|GetSkillData)))))
    (Variables|Default|SetcoolTimeHandler _returnvalue_6)
    (Class|PrimitiveComponent|SetLinearDamping _hitpoint 25.0)
    (Physics|AddImpulse _hitpoint (* _returnvalue_5 (* 1e+08 (* (* _x _x) (* _x 0.8)))) "None" false)
    (bind _returnvalue_7 (Effects|SpawnEmitteratLocation "/Game/Space/Particle/Blink_Particle.Blink_Particle" _returnvalue_3 (Math|Rotator|MakeRotfromX _returnvalue_5)))
    (Utilities|Time|SetTimerbyFunctionName 0 "SetShipDamping" 1.0)))

(fn ConstructionScript
  (|CallParentFunction))

(fn SetShipDamping
  (Class|PrimitiveComponent|SetLinearDamping (Variables|Default|GetHitPoint) 0.7))