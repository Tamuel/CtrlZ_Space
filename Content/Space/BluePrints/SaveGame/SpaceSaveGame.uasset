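; Save game object for the space game, storing the player ship's state and planet exploration progress.
; SaveUnit packs player skills, part classes, inventory, position, vitals and population into ShipSaveData, which raw getter and setter functions also expose.
; LoadUnit applies classes and location, calls InitializeUnit, then restores current load, durability, energy and population.
; SavePlanet and LoadPlanet store and return passed checks and used explore points.
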(fn SaveUnit
  (params (UserUnit :type Unit%20Object%20Reference))
  (bind _player (Variables|/Game/Space/BluePrints/Unit/Unit.Unit_C|GetPlayer UserUnit))
  (bind _asship_unit (Utilities|Casting|CastToShip_Unit UserUnit)
    (:then
      _)
    (:CastFailed
      _))
  (Variables|DatatoSave|SetShipSaveData (Utilities|Struct|MakeShipData (Variables|/Game/Space/BluePrints/Player/SpacePlayer.SpacePlayer_C|GetTechnicalSkills _player) (Variables|/Game/Space/BluePrints/Player/SpacePlayer.SpacePlayer_C|GetRemnantTechSkillls _player) (Variables|/Game/Space/BluePrints/Player/SpacePlayer.SpacePlayer_C|GetExplorePoint _player) (Variables|/Game/Space/BluePrints/Unit/Unit.Unit_C|GetSkills UserUnit) (Variables|/Game/Space/BluePrints/Unit/Unit.Unit_C|GetWeaponClass UserUnit) (Variables|/Game/Space/BluePrints/Ship/Ship_Unit.Ship_Unit_C|GetEngineClass _asship_unit) (Variables|/Game/Space/BluePrints/Unit/Unit.Unit_C|GetBodyClass UserUnit) (Variables|/Game/Space/BluePrints/Ship/Ship_Unit.Ship_Unit_C|GetCoreClass _asship_unit) (Variables|/Game/Space/BluePrints/Unit/Unit.Unit_C|GetItems UserUnit) (Transformation|GetWorldLocation (Variables|/Game/Space/BluePrints/Unit/Unit.Unit_C|GetPhysicsCore UserUnit)) (Variables|/Game/Space/BluePrints/Destroyable/Destroyable.Destroyable_C|GetCurrentDurability UserUnit) (Variables|/Game/Space/BluePrints/Unit/Unit.Unit_C|GetCurrentEnergy UserUnit) (Variables|/Game/Space/BluePrints/Ship/Ship_Unit.Ship_Unit_C|GetFoods _asship_unit) (Variables|/Game/Space/BluePrints/Unit/Unit.Unit_C|GetCurrentLoadage _asship_unit) (Variables|/Game/Space/BluePrints/Population/Population.Population_C|GetPopulationData (Variables|/Game/Space/BluePrints/Ship/Ship_Unit.Ship_Unit_C|GetPopulation _asship_unit)))))

(fn LoadUnit
  (params (NewUnit :type Unit%20Object%20Reference))
  (bind _shipsavedata (Variables|DatatoSave|GetShipSaveData))
  (bind (_technicalskills _remnanttechskills _explorepoint _skillclasses _weaponclasses _engineclass _bodyclass _coreclass _items _unitposition _currentdurabillity _currentenergy _foods _currentloadage _populationdata) (Utilities|Struct|BreakShipData _shipsavedata))
  (bind _asship_unit (Utilities|Casting|CastToShip_Unit NewUnit))
  (Variables|/Game/Space/BluePrints/Player/SpacePlayer.SpacePlayer_C|SetTechnicalSkills (Variables|/Game/Space/BluePrints/Unit/Unit.Unit_C|GetPlayer _asship_unit) _technicalskills)
  (Variables|/Game/Space/BluePrints/Player/SpacePlayer.SpacePlayer_C|SetRemnantTechSkillls (Variables|/Game/Space/BluePrints/Unit/Unit.Unit_C|GetPlayer _asship_unit) _remnanttechskills)
  (Variables|/Game/Space/BluePrints/Player/SpacePlayer.SpacePlayer_C|SetExplorePoint (Variables|/Game/Space/BluePrints/Unit/Unit.Unit_C|GetPlayer _asship_unit) _explorepoint)
  (Variables|/Game/Space/BluePrints/Unit/Unit.Unit_C|SetSkills _asship_unit _skillclasses)
  (Variables|/Game/Space/BluePrints/Unit/Unit.Unit_C|SetWeaponClass _asship_unit _weaponclasses)
  (Variables|/Game/Space/BluePrints/Unit/Unit.Unit_C|SetBodyClass _asship_unit _bodyclass)
  (Variables|/Game/Space/BluePrints/Ship/Ship_Unit.Ship_Unit_C|SetEngineClass _asship_unit _engineclass)
  (Variables|/Game/Space/BluePrints/Ship/Ship_Unit.Ship_Unit_C|SetCoreClass _asship_unit _coreclass)
  (Variables|/Game/Space/BluePrints/Unit/Unit.Unit_C|SetItems _asship_unit _items)
  (Variables|/Game/Space/BluePrints/Ship/Ship_Unit.Ship_Unit_C|SetFoods _asship_unit _foods)
  (Transformation|SetWorldLocation (Variables|/Game/Space/BluePrints/Unit/Unit.Unit_C|GetPhysicsCore _asship_unit) _unitposition false true)
  (Transformation|SetActorLocation _asship_unit _unitposition false true)
  (Default|InitializeUnit _asship_unit)
  (Variables|/Game/Space/BluePrints/Unit/Unit.Unit_C|SetCurrentLoadage _asship_unit _currentloadage)
  (Variables|/Game/Space/BluePrints/Destroyable/Destroyable.Destroyable_C|SetCurrentDurability _asship_unit _currentdurabillity)
  (Variables|/Game/Space/BluePrints/Unit/Unit.Unit_C|SetCurrentEnergy _asship_unit _currentenergy)
  (Variables|/Game/Space/BluePrints/Population/Population.Population_C|SetPopulationData (Variables|/Game/Space/BluePrints/Ship/Ship_Unit.Ship_Unit_C|GetPopulation _asship_unit) _populationdata))

(fn SaveUnitData
  (params (DataToSave :type Ship%20Data%20Structure))
  (Variables|DatatoSave|SetShipSaveData DataToSave))

(fn LoadUnitData
  (return (Variables|DatatoSave|GetShipSaveData)))

(fn SavePlanet
  (params (PassedCheck :type Array%20of%20Booleans) (UsedExplorePoint :type Integer))
  (for (_array_element _array_index) PassedCheck
    (Utilities|Array|SetArrayElem (.PassedCheck (Utilities|Struct|BreakPlanetData (Variables|DatatoSave|GetPlanetSaveData))) _array_index _array_element true))
  (Variables|DatatoSave|SetPlanetSaveData (Utilities|Struct|MakePlanetData (.PassedCheck (Utilities|Struct|BreakPlanetData (Variables|DatatoSave|GetPlanetSaveData))) UsedExplorePoint)))

(fn LoadPlanet
  (bind _planetsavedata (Variables|DatatoSave|GetPlanetSaveData))
  (bind (_passedcheck _usedexplorepoint) (Utilities|Struct|BreakPlanetData _planetsavedata))
  (return _passedcheck _usedexplorepoint))