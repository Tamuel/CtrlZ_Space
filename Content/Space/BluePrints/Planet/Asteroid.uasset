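; Asteroid Blueprint for the space game: a damageable planet-folder actor with a durability value.
; The Damaged event sets CurrentDurability to the incoming Damage minus the current durability, an operand order that is reversed from a usual health decrement.
; At zero or below it calls AsteroidDestroyed, which only swaps the sphere to a red material without removing the actor.
; BeginPlay, overlap and Tick are empty.
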(event EventBeginPlay)

(event EventActorBeginOverlap
  (params (OtherActor :type Actor%20Object%20Reference)))

(event EventTick
  (params (DeltaSeconds :type Float%20%28single-precision%29)))

(event EventDamaged
  (params (Damage :type Integer) (Location :type Vector :default "0, 0, 0") (OtherActorsOwner :type Actor%20Object%20Reference))
  (bind _output_get (Variables|Default|SetCurrentDurability (- Damage (Variables|Default|GetCurrentDurability))))
  (if (<= _output_get 0)
    (CallFunction|AsteroidDestroyed)))

(fn ConstructionScript
  (|CallParentFunction))

(fn AsteroidDestroyed
  (Rendering|Material|SetMaterial (Variables|Default|GetasteroidSphere) 0 "/Game/Space/Images/Laser/RedMaterial.RedMaterial"))