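; GunBarrel is a weapon barrel actor that yaws in response to an attack point and tracks a charging state.
; RotatetoAttackPoint dots the direction to the target with the actor's forward vector, using the sign to pick the turn direction.
; TurningSpeed scales down linearly as that dot nears zero, easing rotation to a stop where forward is perpendicular to the target.
; Each call applies one unscaled-by-time step, and Discharge only clears IsCharging.
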(event EventRotatetoAttackPoint
  (params (AttackPoint :type Actor%20Object%20Reference))
  (bind _returnvalue (Transformation|GetActorRotation))
  (bind _returnvalue_2 (Transformation|GetActorLocation AttackPoint))
  (bind _returnvalue_3 (Transformation|GetActorLocation))
  (bind _returnvalue_4 (Math|Vector|GetForwardVector _returnvalue))
  (bind _returnvalue_5 (- _returnvalue_2 _returnvalue_3))
  (bind _returnvalue_6 (Math|Vector|Normalize _returnvalue_4))
  (bind _returnvalue_7 (Math|Vector|Normalize _returnvalue_5))
  (bind _returnvalue_8 (Math|Vector|DotProduct _returnvalue_7 _returnvalue_6))
  (bind _returnvalue_9 (Math|Float|Absolute(Float) _returnvalue_8))
  (Utilities|IsValid AttackPoint
    (:Is%20Valid
      (if (> _returnvalue_9 0.2)
        (Variables|Default|SetPercentage 1.0)
        (else
          (Variables|Default|SetPercentage (* _returnvalue_9 5.0))))
      (if (> 0.0 _returnvalue_8)
        (Transformation|AddActorLocalRotation (Math|Rotator|MakeRotator 0.0 0.0 (- 0.0 (* (Variables|Default|GetPercentage) (Variables|Default|GetTurningSpeed)))) false false)
        (else
          (Transformation|AddActorLocalRotation (Math|Rotator|MakeRotator 0.0 0.0 (* (Variables|Default|GetPercentage) (Variables|Default|GetTurningSpeed))) false false))))))

(event EventTick
  (params (DeltaSeconds :type Float%20%28single-precision%29))
  (|CallParentFunction 0.0))

(event EventBeginPlay
  (|CallParentFunction))

(fn ConstructionScript)

(fn Discharge
  (Variables|Default|SetisCharging false))