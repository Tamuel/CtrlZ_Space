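; SpacePlayer is the player input Blueprint for the space game, relaying movement, skill and weapon controls to OwnUnit.
; Skill and weapon auto-toggle actions each derive a slot index by switching on the pressed key's display name.
; Left click draws the unit's weapon assistance line, and a separate action toggles the mouse cursor.
; Tick shows queued InteractionWidgets one at a time; confirm or cancel calls the widget's handler, then removes it.
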(event EventBeginPlay)

(event EventActorBeginOverlap
  (params (OtherActor :type Actor%20Object%20Reference)))

(event EventTick
  (params (DeltaSeconds :type Float%20%28single-precision%29))
  (bind _interactionwidgets (Variables|Default|GetInteractionWidgets))
  (if (and (!= (Utilities|Array|Length _interactionwidgets) 0) (not (Variables|Default|GetInteractionUIIsOn)))
    (bind _output_get (Variables|Default|SetCurrentInteractionUI (Utilities|Array|Get(acopy) _interactionwidgets)))
    (UserInterface|Viewport|AddtoViewport _output_get 0)
    (Variables|Default|SetInteractionUIIsOn true)))

(event Input|ActionEvents|InputActionActivateSkill
  (params (Key :type Key%20Structure :default "AnyKey"))
  (bind _ownunit (Variables|Default|GetOwnUnit))
  ;[1 1 1] Use Skills
  (:Pressed
    (switch string (Utilities|String|ToString(Text) (Class|KismetInputLibrary|KeyGetDisplayName Key))
      (:Q
        (Default|UseSkill _ownunit))
      (:E
        (Default|UseSkill _ownunit 1))
      (:1
        (Default|UseSkill _ownunit 2))
      (:2
        (Default|UseSkill _ownunit 3))
      (:3
        (Default|UseSkill _ownunit 4))
      (:4
        (Default|UseSkill _ownunit 5))
      (:5
        (Default|UseSkill _ownunit 6)))))

(event Input|ActionEvents|InputActionInteraction
  (params (Key :type Key%20Structure :default "AnyKey"))
  (:Pressed
    (if (Variables|Default|GetInteractionUIIsOn)
      (Variables|Default|SetInteractionUIIsOn false)
      (Default|Interaction (Variables|Default|GetCurrentInteractionUI))
      (Widget|RemovefromParent (Variables|Default|GetCurrentInteractionUI))
      (Utilities|Array|RemoveItem (Variables|Default|GetInteractionWidgets) (Variables|Default|GetCurrentInteractionUI))
      (Variables|Default|SetCurrentInteractionUI 0))))

(event Input|ActionEvents|InputActionToggleMouse
  (params (Key :type Key%20Structure :default "AnyKey"))
  (bind _returnvalue (Game|GetPlayerController 0))
  ;[1 1 1] Show Mouse
  (:Pressed
    (if (Variables|/Script/Engine.PlayerController|GetbShowMouseCursor _returnvalue)
      (Variables|/Script/Engine.PlayerController|SetbShowMouseCursor _returnvalue false)
      (else
        (Variables|/Script/Engine.PlayerController|SetbShowMouseCursor _returnvalue true)))))

(event Input|ActionEvents|InputActionToggleWeaponInWeapon
  (params (Key :type Key%20Structure :default "AnyKey"))
  (bind _ownunit (Variables|Default|GetOwnUnit))
  ;[1 1 1] Toggle Weapon in Auto
  (:Pressed
    (switch string (Utilities|String|ToString(Text) (Class|KismetInputLibrary|KeyGetDisplayName Key))
      (:F1
        (Default|ToggleWeaponinAuto _ownunit))
      (:F2
        (Default|ToggleWeaponinAuto _ownunit 1))
      (:F3
        (Default|ToggleWeaponinAuto _ownunit 2))
      (:F4
        (Default|ToggleWeaponinAuto _ownunit 3))
      (:F5
        (Default|ToggleWeaponinAuto _ownunit 4))
      (:F6
        (Default|ToggleWeaponinAuto _ownunit 5))
      (:F7
        (Default|ToggleWeaponinAuto _ownunit 6))
      (:F8
        (Default|ToggleWeaponinAuto _ownunit 7)))))

(event Input|ActionEvents|InputActionInteractionCancel
  (params (Key :type Key%20Structure :default "AnyKey"))
  (:Pressed
    (if (Variables|Default|GetInteractionUIIsOn)
      (Variables|Default|SetInteractionUIIsOn false)
      (Default|InteractionCancel (Variables|Default|GetCurrentInteractionUI))
      (Widget|RemovefromParent (Variables|Default|GetCurrentInteractionUI))
      (Utilities|Array|RemoveItem (Variables|Default|GetInteractionWidgets) (Variables|Default|GetCurrentInteractionUI))
      (Variables|Default|SetCurrentInteractionUI 0))))

(event Input|AxisEvents|InputAxisForwardAndBackward
  (params (AxisValue :type Float%20%28single-precision%29))
  (Default|MoveForwardorBackward (Variables|Default|GetOwnUnit) AxisValue))

(event Input|AxisEvents|InputAxisLeftAndRight
  (params (AxisValue :type Float%20%28single-precision%29))
  (Default|TurnLeftorRight (Variables|Default|GetOwnUnit) AxisValue))

(event Input|MouseEvents|LeftMouseButton
  (params (Key :type Key%20Structure :default "AnyKey"))
  (:Pressed
    (Default|DrawWeaponAssistanceLine (Variables|Default|GetOwnUnit))))

(fn ConstructionScript)