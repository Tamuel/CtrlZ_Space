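; Toggleable barrier skill that flags its owner for damage-to-energy and energy drain while active.
; ActiveSkill lazily spawns and attaches a BarrierCollider, then toggles the barrier, updating skill state, collider overlaps and actor tick.
; Turning on also spawns an attached InitializeBarrier actor.
; Tick drains owner energy each frame; at zero it shuts the barrier off and disables the skill, with a cooldown timer calling EnableSkill.
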(event EventActiveSkill
  (bind _self self)
  (Utilities|IsValid (Variables|Default|GetBarrierCollider)
    (:Is%20Valid
      _)
    (:Is%20Not%20Valid
      (bind _returnvalue (Game|SpawnActorfromClass "/Game/Space/BluePrints/Skills/Barrier/BarrierCollider.BarrierCollider_C" (Math|Transform|MakeTransform (Transformation|GetActorLocation _self) (Transformation|GetActorRotation _self) "4.000000,4.000000,4.000000") false 0 0))
      (bind _output_get (Variables|Default|SetBarrierCollider _returnvalue))
      (Variables|/Game/Space/BluePrints/Skills/Barrier/BarrierCollider.BarrierCollider_C|SetSkillData _output_get (Variables|Default|GetSkillData))
      (Class|Actor|AttachRootComponenttoActor _output_get self "None" "KeepWorldPosition" true)))
  (if (.IsActive (Utilities|Struct|BreakSkillStructure (Variables|Default|GetSkillData)))
    (CallFunction|TurnOffBarrier)
    (else
      (CallFunction|TurnonBarrier))))

(event EventBeginPlay)

(event Collision|EventActorBeginOverlap
  (params (OtherActor :type Actor%20Object%20Reference)))

(event EventTick
  (params (DeltaSeconds :type Float%20%28single-precision%29))
  (Default|DecreaseEnergy (.Owner (Utilities|Struct|BreakSkillStructure (Variables|Default|GetSkillData))) 2)
  (if (== 0 (Variables|/Game/Space/BluePrints/Ship/Ship.Ship_C|GetCurrentEnergy (.Owner (Utilities|Struct|BreakSkillStructure (Variables|Default|GetSkillData)))))
    (CallFunction|TurnOffBarrier)
    (Variables|Default|SetSkillData (Utilities|Struct|MakeSkillStructure (.CoolTime (Utilities|Struct|BreakSkillStructure (Variables|Default|GetSkillData))) false true (.EnergyConsumption (Utilities|Struct|BreakSkillStructure (Variables|Default|GetSkillData))) (.Icon_Enable (Utilities|Struct|BreakSkillStructure (Variables|Default|GetSkillData))) (.Icon_Disable (Utilities|Struct|BreakSkillStructure (Variables|Default|GetSkillData))) (.Icon_On (Utilities|Struct|BreakSkillStructure (Variables|Default|GetSkillData))) (.Owner (Utilities|Struct|BreakSkillStructure (Variables|Default|GetSkillData)))))
    (Utilities|Time|SetTimerbyFunctionName 0 "EnableSkill" (.CoolTime (Utilities|Struct|BreakSkillStructure (Variables|Default|GetSkillData))))))

(fn ConstructionScript
  (|CallParentFunction))

(fn TurnonBarrier
  (bind _barriercollider (Variables|Default|GetBarrierCollider))
  (Variables|Default|SetSkillData (Utilities|Struct|MakeSkillStructure (.CoolTime (Utilities|Struct|BreakSkillStructure (Variables|Default|GetSkillData))) true (.Disable (Utilities|Struct|BreakSkillStructure (Variables|Default|GetSkillData))) (.EnergyConsumption (Utilities|Struct|BreakSkillStructure (Variables|Default|GetSkillData))) (.Icon_Enable (Utilities|Struct|BreakSkillStructure (Variables|Default|GetSkillData))) (.Icon_Disable (Utilities|Struct|BreakSkillStructure (Variables|Default|GetSkillData))) (.Icon_On (Utilities|Struct|BreakSkillStructure (Variables|Default|GetSkillData))) (.Owner (Utilities|Struct|BreakSkillStructure (Variables|Default|GetSkillData)))))
  (Variables|/Game/Space/BluePrints/Ship/Ship.Ship_C|SetDamageToEnergy (.Owner (Utilities|Struct|BreakSkillStructure (Variables|Default|GetSkillData))) true)
  (Variables|/Game/Space/BluePrints/Ship/Ship.Ship_C|SetDrainEnergy (.Owner (Utilities|Struct|BreakSkillStructure (Variables|Default|GetSkillData))) true)
  (bind _returnvalue (Game|SpawnActorfromClass "/Game/Space/BluePrints/Skills/Barrier/InitializeBarrier.InitializeBarrier_C" (Math|Transform|MakeTransform (Transformation|GetActorLocation (.Owner (Utilities|Struct|BreakSkillStructure (Variables|Default|GetSkillData)))) "0, 0, 0" "4.000000,4.000000,4.000000") true 0 0))
  (Class|Actor|AttachRootComponenttoActor _returnvalue self "None" "KeepWorldPosition" true)
  (Variables|/Game/Space/BluePrints/Skills/Barrier/BarrierCollider.BarrierCollider_C|SetSkillData _barriercollider (Utilities|Struct|MakeSkillStructure 0.0 true false 0 0 0 0 (.Owner (Utilities|Struct|BreakSkillStructure (Variables|Default|GetSkillData)))))
  (Variables|/Script/Engine.PrimitiveComponent|SetbGenerateOverlapEvents (Variables|/Game/Space/BluePrints/Skills/Barrier/BarrierCollider.BarrierCollider_C|GetSphere _barriercollider) true)
  (Actor|Tick|SetActorTickEnabled true))

(fn TurnOffBarrier
  (bind _barriercollider (Variables|Default|GetBarrierCollider))
  (Variables|Default|SetSkillData (Utilities|Struct|MakeSkillStructure (.CoolTime (Utilities|Struct|BreakSkillStructure (Variables|Default|GetSkillData))) false (.Disable (Utilities|Struct|BreakSkillStructure (Variables|Default|GetSkillData))) (.EnergyConsumption (Utilities|Struct|BreakSkillStructure (Variables|Default|GetSkillData))) (.Icon_Enable (Utilities|Struct|BreakSkillStructure (Variables|Default|GetSkillData))) (.Icon_Disable (Utilities|Struct|BreakSkillStructure (Variables|Default|GetSkillData))) (.Icon_On (Utilities|Struct|BreakSkillStructure (Variables|Default|GetSkillData))) (.Owner (Utilities|Struct|BreakSkillStructure (Variables|Default|GetSkillData)))))
  (Variables|/Game/Space/BluePrints/Ship/Ship.Ship_C|SetDamageToEnergy (.Owner (Utilities|Struct|BreakSkillStructure (Variables|Default|GetSkillData))) false)
  (Variables|/Game/Space/BluePrints/Ship/Ship.Ship_C|SetDrainEnergy (.Owner (Utilities|Struct|BreakSkillStructure (Variables|Default|GetSkillData))) false)
  (Variables|/Game/Space/BluePrints/Skills/Barrier/BarrierCollider.BarrierCollider_C|SetSkillData _barriercollider (Utilities|Struct|MakeSkillStructure 0.0 false false 0 0 0 0 (.Owner (Utilities|Struct|BreakSkillStructure (Variables|Default|GetSkillData)))))
  (Variables|/Script/Engine.PrimitiveComponent|SetbGenerateOverlapEvents (Variables|/Game/Space/BluePrints/Skills/Barrier/BarrierCollider.BarrierCollider_C|GetSphere _barriercollider) false)
  (Actor|Tick|SetActorTickEnabled false))