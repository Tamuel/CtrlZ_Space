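; Base Blueprint for a ship-mounted weapon in a space game.
; InitializeWeapon claims the next free slot on the owning ship, registers the weapon and updates the ship's minimum weapon range.
; While equipped and the ship has an attack point, Tick calls rotation toward the weapon's own target.
; Outside player control, it also draws an assistance line or clears out-of-range targets; rotation and line functions are empty stubs.
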(event EventBeginPlay)

(event EventActorBeginOverlap
  (params (OtherActor :type Actor%20Object%20Reference)))

(event EventTick
  (params (DeltaSeconds :type Float%20%28single-precision%29))
  (bind _itemdata (Variables|Default|GetitemData))
  (bind _owner (Utilities|Struct|BreakItemStructure _itemdata))
  (if (and (Variables|Default|GetisEquiped) (Utilities|IsValid _owner))
    ;[1 1 1] If Attack Point of Ship is valid
    (if (Utilities|IsValid (Variables|/Game/Space/BluePrints/Unit/Unit.Unit_C|GetAttackPoint _owner))
      ;[1 1 1] Rotate to Attack Point (When equipped)
      (if (Variables|Default|GetIsInControl)
        (CallFunction|RotatetoAttackPoint (Variables|Reference|GetAttackPoint))
        (else
          (Utilities|IsValid (Variables|Reference|GetAttackPoint)
            (:Is%20Valid
              (CallFunction|RotatetoAttackPoint (Variables|Reference|GetAttackPoint))
              (bind _isinrange (CallFunction|EnemyIsinRange))
              (if _isinrange
                (CallFunction|DrawAssistanceLine)
                (else
                  (Variables|Reference|SetAttackPoint 0))))))))))

(fn ConstructionScript)

(fn EnemyIsinRange
  (bind _output_get (Variables|Default|SetAttackPointIsInRange (<= (Math|Vector|VectorLength (- (Transformation|GetActorLocation (Variables|Reference|GetAttackPoint)) (Transformation|GetActorLocation self))) (* (Variables|Properties|GetFireRange) 1e+02))))
  (return _output_get))

(fn RotatetoAttackPoint
  (params (AttackPoint :type Actor%20Object%20Reference)))

(fn DrawAssistanceLine)

(fn InitializeWeapon
  (bind _itemdata (Variables|Default|GetitemData))
  (bind _itemdata_2 (Variables|Default|GetitemData))
  (bind _owner (Utilities|Struct|BreakItemStructure _itemdata))
  (bind _owner_2 (Utilities|Struct|BreakItemStructure _itemdata_2))
  (bind _weapons (Variables|/Game/Space/BluePrints/Unit/Unit.Unit_C|GetWeapons _owner_2))
  (bind _returnvalue (Utilities|Array|Length _weapons))
  ;[1 1 1] Equip Weapon and Set Weapon Position at ship
  (if (and (not (Variables|Default|GetisEquiped)) (Utilities|IsValid _owner_2))
    (if (> (Variables|/Game/Space/BluePrints/Unit/Unit.Unit_C|GetMaxNumberOfWeapons _owner_2) _returnvalue)
      (Variables|Default|SetPositionOfWeapon _returnvalue)
      (Variables|Default|SetisEquiped true)
      (Utilities|Array|Add (Variables|/Game/Space/BluePrints/Unit/Unit.Unit_C|GetWeapons _owner) self)
      (Default|SetMinRangeOfWeapon _owner))))