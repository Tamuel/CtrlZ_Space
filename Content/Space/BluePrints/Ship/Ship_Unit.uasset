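; Ship unit for the space game that spawns core and engine parts, copies their stats, and turns axis input into movement that drains energy.
; For the player, a timer-repeated sphere trace with line-of-sight checks finds nearby units and rebuilds minimap markers.
; Units of other alliances are distance-sorted and distributed across WeaponsOutControl as auto-targets.
; On destruction it spawns an explosion, destroys body and weapons, and drops loot.
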(event EventBeginPlay
  (CallFunction|AttachCore)
  (CallFunction|AttachEngine)
  (|CallParentFunction)
  (if (Variables|Default|GetisPlayer)
    (bind _returnvalue (UserInterface|CreateWidget "/Game/Space/UI/MainUI.MainUI_C" (Game|GetPlayerController 0)))
    (UserInterface|Viewport|AddtoViewport _returnvalue 0)
    (CallFunction|SearchUnitsinRange)))

(event EventActorBeginOverlap
  (params (OtherActor :type Actor%20Object%20Reference)))

(event EventTick
  (params (DeltaSeconds :type Float%20%28single-precision%29))
  (|CallParentFunction DeltaSeconds))

(event EventDestroyEvent
  (Variables|Default|SetCurrentForwardSpeed 0.0)
  (Variables|Default|SetCurrentTurningSpeed 0.0)
  (Effects|SpawnEmitteratLocation "/Game/Space/Particle/P_Explosion.P_Explosion" (Transformation|GetActorLocation self))
  (Class|Pawn|DetachfromControllerPendingDestroy)
  (Actor|DestroyActor (Variables|Default|GetBodyIns))
  (Actor|DestroyActor (Variables|Default|GetWeapons))
  (CallFunction|DropItem (Utilities|Array|MakeArray "/Game/Space/BluePrints/Item/Iron.Iron_C" "/Game/Space/BluePrints/Weapons/Laser/SmallLaserGun.SmallLaserGun_C"))
  (Actor|DestroyActor))

(event Input|AxisEvents|InputAxisForwardAndBackward
  (params (AxisValue :type Float%20%28single-precision%29))
  (if (!= AxisValue 0.0)
    (CallFunction|MoveForwardorBackward AxisValue)
    (CallFunction|DecreaseEnergy (Variables|/Game/Space/BluePrints/Ship/ShipEngine.ShipEngine_C|GetEnergyDecreaseRate (Variables|ShipComponent|GetShipEngineIns)))))

(event Input|AxisEvents|InputAxisLeftAndRight
  (params (AxisValue :type Float%20%28single-precision%29))
  (if (!= AxisValue 0.0)
    (CallFunction|TurnLeftorRight AxisValue)
    (CallFunction|DecreaseEnergy (Variables|/Game/Space/BluePrints/Ship/ShipEngine.ShipEngine_C|GetEnergyDecreaseRate (Variables|ShipComponent|GetShipEngineIns)))))

(event Input|MouseEvents|LeftMouseButton
  (params (Key :type Key%20Structure :default "AnyKey"))
  (:Pressed
    (CallFunction|DrawWeaponAssistanceLine)))

(fn ConstructionScript
  (|CallParentFunction))

(fn SearchUnitsinRange
  (bind _self self)
  (bind _minimappos (Variables|Default|GetMiniMapPos))
  (bind _returnvalue (Transformation|GetActorLocation _self))
  (for _array_element _minimappos
    (Widget|RemovefromParent _array_element))
  (Utilities|Array|Clear _minimappos)
  (Utilities|Array|Clear (Variables|Default|GetUnitsAroundMe))
  (bind _output_get (Variables|Default|SetMyLocation _returnvalue))
  (bind _outhits (Collision|MultiSphereTraceForObjects _output_get (+ _returnvalue "0, 0,100.000000") (* (Variables|Default|GetDetectingRange) 1e+02) (Variables|Default|GetDesiredObjectTypes) false 0 "None"))
  (for _array_element_2 _outhits
    (bind _outhit (Collision|LineTraceByChannel (Variables|Default|GetMyLocation) (Transformation|GetActorLocation (.HitActor (Collision|BreakHitResult _array_element_2))) "TraceTypeQuery2" false 0 "None"))
    (if (== (.HitActor (Collision|BreakHitResult _outhit)) (.HitActor (Collision|BreakHitResult _array_element_2)))
      (bind _asunit (Utilities|Casting|CastToUnit (.HitActor (Collision|BreakHitResult _outhit))))
      (Utilities|Array|Add (Variables|Default|GetUnitsAroundMe) _asunit)
      (bind _returnvalue_2 (UserInterface|CreateWidget "/Game/Space/UI/MiniMapPosition.MiniMapPosition_C"))
      (Variables|/Game/Space/UI/MiniMapPosition.MiniMapPosition_C|SetUnit _returnvalue_2 _asunit)
      (Utilities|Array|Add (Variables|Default|GetMiniMapPos) _returnvalue_2)
      (UserInterface|Viewport|AddtoViewport _returnvalue_2 0)))
  (CallFunction|SearchAutoWeaponTarget)
  (Utilities|Time|SetTimerbyFunctionName 0 "SearchUnitsInRange" 1.5))

(fn SearchAutoWeaponTarget
  (bind _enemyunitsaroundme (Variables|Default|GetEnemyUnitsAroundMe))
  (bind _weaponsoutcontrol (Variables|Default|GetWeaponsOutControl))
  ;[1 1 1] Search Enemies
  (Utilities|Array|Clear (Variables|Default|GetEnemyUnitsAroundMe))
  (if (!= (Utilities|Array|Length (Variables|Default|GetWeaponsOutControl)) 0)
    (for _array_element (Variables|Default|GetUnitsAroundMe)
      (if (!= (Variables|/Game/Space/BluePrints/Unit/Unit.Unit_C|GetAlliance _array_element) (Variables|Default|GetAlliance))
        (Utilities|Array|Add (Variables|Default|GetEnemyUnitsAroundMe) _array_element)))
    (CallFunction|SortingEnemiesbyDistance)
    (if (>= (Utilities|Array|Length _enemyunitsaroundme) (Utilities|Array|Length _weaponsoutcontrol))
      (for (_array_element_2 _array_index) _weaponsoutcontrol
        (Variables|/Game/Space/BluePrints/Weapons/Weapon.Weapon_C|SetAttackPoint _array_element_2 (Utilities|Array|Get(acopy) _enemyunitsaroundme _array_index)))
      (else
        (for (_array_element_3 _array_index_2) _weaponsoutcontrol
          (Variables|/Game/Space/BluePrints/Weapons/Weapon.Weapon_C|SetAttackPoint _array_element_3 (Utilities|Array|Get(acopy) _enemyunitsaroundme (Math|Integer|%(Integer) _array_index_2 (Utilities|Array|Length _enemyunitsaroundme)))))))))

(fn SortingEnemiesbyDistance
  (bind _enemyunitsaroundme (Variables|Default|GetEnemyUnitsAroundMe))
  (bind _returnvalue (Utilities|Array|Length _enemyunitsaroundme))
  (for _index (range 0 _returnvalue)
    (Utilities|IsValid (Utilities|Array|Get(acopy) _enemyunitsaroundme _index)
      (:Is%20Valid
        (LocalVariables|SetMinLength (Math|Vector|VectorLength (- (Transformation|GetActorLocation (Utilities|Array|Get(acopy) _enemyunitsaroundme _index)) (Transformation|GetActorLocation self))))
        (for _index_2 (range (+ _index 1) _returnvalue)
          (Utilities|IsValid (Utilities|Array|Get(acopy) _enemyunitsaroundme _index_2)
            (:Is%20Valid
              (if (> (LocalVariables|GetMinLength) (Math|Vector|VectorLength (- (Transformation|GetActorLocation (Utilities|Array|Get(acopy) _enemyunitsaroundme _index_2)) (Transformation|GetActorLocation self))))
                (LocalVariables|SetMinLength (Math|Vector|VectorLength (- (Transformation|GetActorLocation (Utilities|Array|Get(acopy) _enemyunitsaroundme _index_2)) (Transformation|GetActorLocation self))))
                (LocalVariables|SetMinIndex _index_2)))))
        (bind _output_get (LocalVariables|SetTempActor (Utilities|Array|Get(acopy) _enemyunitsaroundme (LocalVariables|GetMinIndex))))
        (Utilities|Array|SetArrayElem _enemyunitsaroundme (LocalVariables|GetMinIndex) (Utilities|Array|Get(acopy) _enemyunitsaroundme _index))
        (Utilities|Array|SetArrayElem _enemyunitsaroundme _index _output_get)))))

(fn AttachCore
  (bind _coreclass (Variables|ShipComponent|GetCoreClass))
  (if (Utilities|IsValidClass _coreclass)
    (bind _returnvalue (Game|SpawnActorfromClass _coreclass (Math|Transform|MakeTransform "0, 0, 0") "AlwaysSpawn" 0 0))
    (bind _output_get (Variables|ShipComponent|SetShipCoreIns _returnvalue))
    (Variables|/Game/Space/BluePrints/Unit/UnitAttachable.UnitAttachable_C|SetOwnerUnit _returnvalue self)
    (CallFunction|AddItem _returnvalue)
    (Class|Actor|AttachRootComponenttoActor _output_get self "None" "SnapToTarget" true)
    (Variables|Default|SetMaxEnergy (Variables|/Game/Space/BluePrints/Ship/ShipCore.ShipCore_C|GetMaxEnergy (Variables|ShipComponent|GetShipCoreIns)))
    (Variables|Default|SetEnergyChargeRate (Variables|/Game/Space/BluePrints/Ship/ShipCore.ShipCore_C|GetEnergyChargeRate (Variables|ShipComponent|GetShipCoreIns)))))

(fn AttachEngine
  (bind _engineclass (Variables|ShipComponent|GetEngineClass))
  (if (Utilities|IsValidClass _engineclass)
    (bind _returnvalue (Game|SpawnActorfromClass _engineclass (Math|Transform|MakeTransform "0, 0, 0") "AlwaysSpawn" 0 0))
    (bind _output_get (Variables|ShipComponent|SetShipEngineIns _returnvalue))
    (Variables|/Game/Space/BluePrints/Unit/UnitAttachable.UnitAttachable_C|SetOwnerUnit _returnvalue self)
    (CallFunction|AddItem _returnvalue)
    (Class|Actor|AttachRootComponenttoActor _output_get self "None" "SnapToTarget" true)
    (Variables|Default|SetmaxSpeed (Variables|/Game/Space/BluePrints/Ship/ShipEngine.ShipEngine_C|GetMaxSpeed (Variables|ShipComponent|GetShipEngineIns)))
    (Variables|Default|SetminSpeed (Variables|/Game/Space/BluePrints/Ship/ShipEngine.ShipEngine_C|GetMinSpeed (Variables|ShipComponent|GetShipEngineIns)))
    (Variables|Default|SetTurningSpeed (Variables|/Game/Space/BluePrints/Ship/ShipEngine.ShipEngine_C|GetTurningSpeed (Variables|ShipComponent|GetShipEngineIns)))
    (Variables|Default|SetAcceleration (Variables|/Game/Space/BluePrints/Ship/ShipEngine.ShipEngine_C|GetAcceleration (Variables|ShipComponent|GetShipEngineIns)))
    (Variables|Default|SetMaxTurnSpeed (Variables|/Game/Space/BluePrints/Ship/ShipEngine.ShipEngine_C|GetMaxTurningSpeed (Variables|ShipComponent|GetShipEngineIns)))))